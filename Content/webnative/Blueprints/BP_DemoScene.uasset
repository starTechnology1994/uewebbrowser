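; Demo scene actor for the WebNative browser plugin, hosting a local HTML page in a viewport widget alongside interactive 3D content.
; JSON-taking functions spawn primitive meshes that follow the cursor via traces until mouse release, or reposition the player's view.
; In the transparent overlay demo, input fires physics spheres, reloads and toggles a panel, sending ammo and panel messages to JavaScript.
; Tick also oscillates a cube sinusoidally.
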(event EventBeginPlay
  (bind _returnvalue (Game|GetPlayerController 0))
  (Development|ExecuteConsoleCommand (Utilities|String|Append "r.SetRes " "1706" "x" "1066" "w") _returnvalue)
  (Input|SetInputModeGameandUI _returnvalue 0 "DoNotLock" false false)
  (Variables|/Script/Engine.PlayerController|SetbShowMouseCursor _returnvalue true)
  (bind _returnvalue_2 (UserInterface|CreateWidget "/WebNativeBrowser/webnative/UMG/BP_WebNative.BP_WebNative_C"))
  (Variables|Default|SetWeb%20Native (Variables|/WebNativeBrowser/webnative/UMG/BP_WebNative.BP_WebNative_C|GetWebNative _returnvalue_2))
  (UserInterface|Viewport|AddtoViewport _returnvalue_2 0)
  (Class|WebNativeBrowserWidget|LoadURL (Variables|Default|GetWeb%20Native) (Class|BlueprintPathsLibrary|ConvertRelativePathtoFull (Class|BlueprintPathsLibrary|Combine (Utilities|Array|MakeArray (Class|BlueprintPathsLibrary|ProjectPluginsDir) "WebNativeBrowser/Content/webnative" "html" "Index.html")))))

(event EventTick
  (params (DeltaSeconds :type Float%20%28single-precision%29))
  (Demo3|DragingModel)
  (Demo3|PingPong DeltaSeconds))

(event Input|KeyboardEvents|R
  (params (Key :type Key%20Structure :default "None"))
  (:Pressed
    (Demo10|Reload)))

(event Input|MouseEvents|LeftMouseButton
  (params (Key :type Key%20Structure :default "None"))
  (:Pressed
    (Demo10|Fire))
  (:Released
    (Demo3|DrapModel)))

(event Input|KeyboardEvents|Escape
  (params (Key :type Key%20Structure :default "None"))
  (:Pressed
    (Demo10|TogglePanel)))

(fn ConstructionScript)

(fn DragStartModel
  (params (dragMes :type String%20%28by%20ref%29))
  (bind _returnvalue (Game|GetPlayerController 0))
  (bind (_worldlocation _worlddirection) (Game|Player|ConvertMouseLocationToWorldSpace _returnvalue))
  (Class|WebNativeBrowserWidget|SetFocustoGameViewport (Variables|Default|GetWeb%20Native))
  (if (and (Variables|Drag|GetisDraging) (Utilities|IsValid (Variables|Drag|GetdragActor)))
    (Actor|DestroyActor (Variables|Drag|GetdragActor)))
  (bind (_outhit _returnvalue_2) (Collision|LineTraceByChannel _worldlocation (+ (* _worlddirection "100000.000000,100000.000000,100000.000000") _worldlocation) "TraceTypeQuery1" true 0 "None"))
  (bind _outjsonobject (Class|JsonBlueprintFunctionLibrary|FromString dragMes))
  (bind _outvalue (|GetJsonField _outjsonobject "modelName"))
  (bind _returnvalue_3 (Game|SpawnActorfromClass "/Script/Engine.StaticMeshActor" (Math|Transform|MakeTransform (Math|Vector|SelectVector (.Location (Collision|BreakHitResult _outhit)) (+ _worldlocation (* _worlddirection (Variables|Drag|GetdefaultDistance))) _returnvalue_2) "0, 0, 0" "1.000000,1.000000,1.000000") "AlwaysSpawn" 0 0))
  (Transformation|SetMobility _returnvalue_3 "Movable")
  (Utilities|FlowControl|Sequence
    (:then_0
      (switch string _outvalue
        (:Cube
          (Components|StaticMesh|SetStaticMesh (Variables|/Script/Engine.StaticMeshActor|GetStaticMeshComponent _returnvalue_3) "/Engine/BasicShapes/Cube.Cube"))
        (:Sphere
          (Components|StaticMesh|SetStaticMesh (Variables|/Script/Engine.StaticMeshActor|GetStaticMeshComponent _returnvalue_3) "/Engine/BasicShapes/Sphere.Sphere"))
        (:Cylinder
          (Components|StaticMesh|SetStaticMesh (Variables|/Script/Engine.StaticMeshActor|GetStaticMeshComponent _returnvalue_3) "/Engine/BasicShapes/Cylinder.Cylinder"))
        (:Cone
          (Components|StaticMesh|SetStaticMesh (Variables|/Script/Engine.StaticMeshActor|GetStaticMeshComponent _returnvalue_3) "/Engine/BasicShapes/Cone.Cone"))
        (:Plane
          (Components|StaticMesh|SetStaticMesh (Variables|/Script/Engine.StaticMeshActor|GetStaticMeshComponent _returnvalue_3) "/Engine/BasicShapes/Plane.Plane"))))
    (:then_1
      (bind _output_get (Variables|Drag|SetdragActor _returnvalue_3))
      (Collision|SetActorEnableCollision _output_get false)
      (Variables|Drag|SetisDraging true))))

(fn DragingModel
  (bind _web_native (Variables|Default|GetWeb%20Native))
  (bind _defaultdistance (Variables|Drag|GetdefaultDistance))
  (bind _outscreenpos (Class|WebNativeBrowserWidget|GetRawPlatformCursorPos _web_native))
  (bind (_outworldpos _outworlddir) (Class|WebNativeBrowserWidget|DeprojectCursortoWorld _web_native _outscreenpos))
  (bind _returnvalue (* _outworlddir _defaultdistance))
  (if (and (Variables|Drag|GetisDraging) (Utilities|IsValid (Variables|Drag|GetdragActor)))
    (bind (_outhit _returnvalue_2) (Collision|LineTraceByChannel _outworldpos (+ _outworldpos _returnvalue) "TraceTypeQuery1" true 0 "None"))
    (Transformation|SetActorLocation (Variables|Drag|GetdragActor) (Math|Vector|SelectVector (+ (.Location (Collision|BreakHitResult _outhit)) (Math|Vector|MakeVector 0.0 0.0 (.z (.BoxExtent (Collision|GetActorBounds (Variables|Drag|GetdragActor) false false))))) _returnvalue _returnvalue_2) false false)))

(fn DrapModel
  (if (and (Variables|Drag|GetisDraging) (Utilities|IsValid (Variables|Drag|GetdragActor)))
    (Collision|SetActorEnableCollision (Variables|Drag|GetdragActor) true)
    (Variables|Drag|SetdragActor 0)))

(fn SwitchView
  (params (viewMes :type String%20%28by%20ref%29))
  (bind _outjsonobject (Class|JsonBlueprintFunctionLibrary|FromString viewMes))
  (bind _outvalue (|GetJsonField _outjsonobject "location"))
  (bind _outvalue_2 (|GetJsonField _outvalue "x"))
  (bind _outvalue_3 (|GetJsonField _outvalue "y"))
  (bind _outvalue_4 (|GetJsonField _outvalue "z"))
  (bind _outvalue_5 (|GetJsonField _outjsonobject "rotation"))
  (bind _outvalue_6 (|GetJsonField _outvalue_5 "roll"))
  (bind _outvalue_7 (|GetJsonField _outvalue_5 "pitch"))
  (bind _outvalue_8 (|GetJsonField _outvalue_5 "yaw"))
  (Transformation|SetActorLocation (Game|Player|GetPlayerPawn 0) (Math|Vector|MakeVector _outvalue_2 _outvalue_3 _outvalue_4) false false)
  (Pawn|SetControlRotation (Game|GetPlayerController 0) (Math|Rotator|MakeRotator _outvalue_6 _outvalue_7 _outvalue_8)))

(fn ClearModel
  (Variables|Drag|SetisDraging false)
  (Variables|Drag|SetdragActor 0))

(fn PingPong
  (params (Delta :type Float%20%28double-precision%29))
  (bind _output_get (Variables|Default|Setangle (+ (Variables|Default|Getangle) (* Delta 2e+02))))
  (Transformation|SetRelativeLocation (Variables|Default|GetCube) (Math|Vector|MakeVector (* (Math|Trig|Sin(Degrees) _output_get) 1e+03) 1.5e+03 1.5e+02) false false))

(fn Fire
  (bind _returnvalue (Game|GetPlayerController 0))
  (bind _returnvalue_2 (Viewport|GetViewportSize))
  (bind _returnvalue_3 (/ _returnvalue_2 "(X=2.000000,Y=2.000000)"))
  (bind (_worldposition _worlddirection) (Class|GameplayStatics|DeprojectScreentoWorld _returnvalue _returnvalue_3))
  (if (Utilities|Enum|Equal(Enum) (Variables|Default|GetcurrentDemo) "10_TransparentOverlay.html")
    (if (> (Variables|TransparentOverlay|Getammo) 0)
      (Math|Integer|DecrementInt (Variables|TransparentOverlay|Getammo)
        (:%20%20
          (bind _returnvalue_4 (Game|SpawnActorfromClass "/Script/Engine.StaticMeshActor" (Math|Transform|MakeTransform _worldposition "0, 0, 0" "0.100000,0.100000,0.100000") "AlwaysSpawn" 0 0))
          (Transformation|SetMobility _returnvalue_4 "Movable")
          (Components|StaticMesh|SetStaticMesh (Variables|/Script/Engine.StaticMeshActor|GetStaticMeshComponent _returnvalue_4) "/Engine/BasicShapes/Sphere.Sphere")
          (Rendering|SetCastShadow (Variables|/Script/Engine.StaticMeshActor|GetStaticMeshComponent _returnvalue_4) false)
          (Physics|SetSimulatePhysics (Variables|/Script/Engine.StaticMeshActor|GetStaticMeshComponent _returnvalue_4) true)
          (Physics|AddImpulseatLocation (Variables|/Script/Engine.StaticMeshActor|GetStaticMeshComponent _returnvalue_4) (* _worlddirection 3e+03) _worldposition "None")))
      (else
        (Variables|TransparentOverlay|Setammo 0)))
    (Class|WebNativeBrowserWidget|SendMessagetoJS (Variables|Default|GetWeb%20Native) "UpdateAmmo" (Utilities|String|Append "{\"ammo\":" (Utilities|String|ToString(Integer) (Variables|TransparentOverlay|Getammo)) "}"))))

(fn TogglePanel
  (if (Utilities|Enum|Equal(Enum) (Variables|Default|GetcurrentDemo) "10_TransparentOverlay.html")
    (Class|WebNativeBrowserWidget|SendMessagetoJS (Variables|Default|GetWeb%20Native) "togglePanel" "{}")))

(fn Reload
  (if (Utilities|Enum|Equal(Enum) (Variables|Default|GetcurrentDemo) "10_TransparentOverlay.html")
    (bind _output_get (Variables|TransparentOverlay|Setammo 30))
    (Class|WebNativeBrowserWidget|SendMessagetoJS (Variables|Default|GetWeb%20Native) "UpdateAmmo" (Utilities|String|Append "{\"ammo\":" (Utilities|String|ToString(Integer) _output_get) "}"))))